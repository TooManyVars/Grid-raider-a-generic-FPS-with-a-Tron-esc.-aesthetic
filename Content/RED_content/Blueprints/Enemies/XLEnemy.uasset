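; XLEnemy is an extra-large enemy Blueprint with high health and a score award, built on a parent class.
; BeginPlay runs the parent logic, then sets its Health and ScoreAwarded values.
; Every Tick runs the parent logic, then searches for all actors tagged "Enemy" and sets EnemyDamage to DamageMultiplier times their count, so damage scales with the number of enemies present.
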(event `self.ReceiveBeginPlay`
  (`parent.ReceiveBeginPlay`)
  (set `self.Health` 1250.0)
  (set `self.ScoreAwarded` 500))

(event `self.ReceiveTick`
  (params (DeltaSeconds :type "Float (single-precision)"))
  (`parent.ReceiveTick` DeltaSeconds)
  (bind _outactors (`GameplayStatics.GetAllActorsWithTag` "Enemy"))
  (set `self.EnemyDamage` (`KismetMathLibrary.Conv_IntToDouble` (* (`self.Damage multiplier`) (`KismetArrayLibrary.Array_Length` _outactors)))))

(fn `UserConstructionScript`
  (`parent.UserConstructionScript`))