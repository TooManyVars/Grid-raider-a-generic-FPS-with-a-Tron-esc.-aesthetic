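; Game mode Blueprint that drives enemy spawning and player respawn.
; On BeginPlay it finds every basic, large, XL and small enemy spawner and starts a looping timer on each to call its spawn function by name.
; Each type has its own interval variable, with the basic one derived from an enemies-per-second rate.
; RespawnPlayer destroys all Enemy actors, then spawns a new Player and possesses it with the first player controller.
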(event `self.ReceiveBeginPlay`
  (`|ExecutionSequence`
    (:`then_0`
      (bind _outactors (`GameplayStatics.GetAllActorsOfClass` "/Game/RED_content/Blueprints/Spawners/WorkingBasicEnemySpawner.WorkingBasicEnemySpawner_C"))
      (for _array_element _outactors
        (bind _output_get (set `self.Spawner` _array_element))
        (`KismetSystemLibrary.K2_SetTimer` _output_get "SpawnEnemy" (/ 1.0 (`self.Enemies per second`)) true)))
    (:`then_1`
      (bind _outactors_2 (`GameplayStatics.GetAllActorsOfClass` "/Game/RED_content/Blueprints/Spawners/WorkingLargeEnemySpawner.WorkingLargeEnemySpawner_C"))
      (for _array_element_2 _outactors_2
        (bind _output_get_2 (set `self.LargeEnemySpawner` _array_element_2))
        (`KismetSystemLibrary.K2_SetTimer` _output_get_2 "Spawn large enemy" (`self.SpawnLargeEnemyTime`) true)))
    (:`then_2`
      (bind _outactors_3 (`GameplayStatics.GetAllActorsOfClass` "/Game/RED_content/Blueprints/Spawners/XLEnemySpawner.XLEnemySpawner_C"))
      (for _array_element_3 _outactors_3
        (bind _output_get_3 (set `self.XL enemy spawner` _array_element_3))
        (`KismetSystemLibrary.K2_SetTimer` _output_get_3 "SpawnEnemy" (`self.SpawnXLEnemyTime`) true)))
    (:`then_3`
      (bind _outactors_4 (`GameplayStatics.GetAllActorsOfClass` "/Game/RED_content/Blueprints/Spawners/SmallEnemySpawner.SmallEnemySpawner_C"))
      (for _array_element_4 _outactors_4
        (bind _output_get_4 (set `self.Small EnemySpawner` _array_element_4))
        (`KismetSystemLibrary.K2_SetTimer` _output_get_4 "SpawnEnemy" (`self.Spawn Small enemy spawn time`) true)))))

(event `RespawnPlayer`
  (bind _outactors (`GameplayStatics.GetAllActorsOfClass` "/Game/RED_content/Blueprints/Enemies/Enemy.Enemy_C"))
  (for _array_element _outactors
    (`self.K2_DestroyActor` _array_element))
  (bind _returnvalue (`|SpawnActorFromClass` "/Game/RED_content/Blueprints/Player/Player.Player_C" (`self.SpawnTransform`) "Undefined" "OverrideRootScale" null null))
  (`Controller.Possess` (`GameplayStatics.GetPlayerController` 0) _returnvalue))

(fn `UserConstructionScript`)