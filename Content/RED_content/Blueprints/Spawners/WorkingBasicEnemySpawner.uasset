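; Enemy spawner Blueprint that places AI pawns at random points inside its SpawnVolume box.
; The SpawnEnemy event counts all world actors of EnemyClass and, while that count is below MaxEnemies, spawns one EnemyType pawn via SpawnAIFromClass.
; The counted class and the spawned class are separate variables, and nothing in this graph calls SpawnEnemy, as BeginPlay and Tick are empty.
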(event `SpawnEnemy`
  (bind _spawnvolume (`self.SpawnVolume`))
  (bind _outactors (`GameplayStatics.GetAllActorsOfClass` (`self.Enemy class`)))
  (if (< (`KismetArrayLibrary.Array_Length` _outactors) (`self.Max enemies`))
    (`AIBlueprintHelperLibrary.SpawnAIFromClass` (`self.EnemyType`) null (`KismetMathLibrary.RandomPointInBoundingBox` (`SceneComponent.K2_GetComponentLocation` _spawnvolume) (`BoxComponent.GetScaledBoxExtent` _spawnvolume)))))

(fn `UserConstructionScript`)