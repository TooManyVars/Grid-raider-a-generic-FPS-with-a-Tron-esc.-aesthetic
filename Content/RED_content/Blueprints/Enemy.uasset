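; Enemy character that damages the player on proximity and can itself be damaged and killed.
; Overlapping DamageBox starts a looping HitPlayer timer at the DPS rate, applying EnemyDamage until the player leaves.
; AffectHealth updates and prints health; on death it disables Pawn and WorldDynamic collision, detaches the controller and destroys the actor after a delay.
; The construction script tints the mesh with EnemyColor through a dynamic material.
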(event `/Game/RED_content/Blueprints/IDamageable.AffectHealth`
  (params (Delta :type "Float (single-precision)"))
  (bind _capsulecomponent (`self.CapsuleComponent`))
  ;[1 1 1] Implementation of IDamagable in which the enemy will take damage and will have the rest of it's health printed to the screen with loiw enough health it will die,
  (`self.RemainingHealth` Delta)
  (`KismetSystemLibrary.PrintString` (`KismetStringLibrary.Conv_DoubleToString` (`self.Health`)) false)
  (`self.CheckDead`)
  (if (`self.IsDead`)
    (`PrimitiveComponent.SetCollisionResponseToChannel` _capsulecomponent "ECC_WorldDynamic" "ECR_Ignore")
    (`PrimitiveComponent.SetCollisionResponseToChannel` _capsulecomponent "ECC_Pawn" "ECR_Ignore")
    (`self.DetachFromControllerPendingDestroy`)
    (`KismetSystemLibrary.Delay` 3.0)
    (`self.K2_DestroyActor`)))

(event `self.DamageBox.OnComponentBeginOverlap`
  (params (OverlappedComponent :type "PrimitiveComponent Object Reference") (OtherActor :type "Actor Object Reference") (OtherComp :type "PrimitiveComponent Object Reference") (OtherBodyIndex :type Integer) (bFromSweep :type Boolean) (SweepResult :type "HitResult Structure (by ref)"))
  ;[1 1 1] Functionality that allows the enemy to hit the player once they enter proximiy.
  (bind _asplayer (cast `/Game/RED_content/Blueprints/Player` OtherActor))
  (set `self.Player character` _asplayer)
  (`KismetSystemLibrary.K2_SetTimer` null "HitPlayer" (/ 1.0 (`self.DPS`)) true))

(event `self.DamageBox.OnComponentEndOverlap`
  (params (OverlappedComponent :type "PrimitiveComponent Object Reference") (OtherActor :type "Actor Object Reference") (OtherComp :type "PrimitiveComponent Object Reference") (OtherBodyIndex :type Integer))
  ;[1 1 1] Functionality that allows the enemy to hit the player once they enter proximiy.
  (if (== OtherActor (`self.Player character`))
    (`KismetSystemLibrary.K2_ClearTimer` null "HitPlayer")))

(event `HitPlayer`
  ;[1 1 1] Functionality that allows the enemy to hit the player once they enter proximiy.
  (`/Game/RED_content/Blueprints/IDamageable.AffectHealth` (`self.Player character`) (`self.EnemyDamage`)))

(fn `UserConstructionScript`
  (bind _returnvalue (`PrimitiveComponent.CreateDynamicMaterialInstance` (`self.Mesh`) 0 null))
  (bind _output_get (set `self.Dynamic Material` _returnvalue))
  (`MaterialInstanceDynamic.SetVectorParameterValue` _output_get "BodyColor" (`self.EnemyColor`)))